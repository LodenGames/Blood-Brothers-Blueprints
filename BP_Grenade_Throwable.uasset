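; Thrown grenade that spawns an explosion after a fixed fuse and damages actors tagged "Person".
; BeginPlay scales inner and outer sphere radii and damage from the player BP_Assault's global and grenade attributes.
; Both spheres start without collision, then enable it at detonation so begin-overlap events apply damage, with the inner amount stacking on the outer.
; The grenade never destroys itself here, so the spheres stay active.
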(event OnComponentBeginOverlap(OuterRadius)
  (params (OverlappedComponent :type Primitive%20Component%20Object%20Reference) (OtherActor :type Actor%20Object%20Reference) (OtherComp :type Primitive%20Component%20Object%20Reference) (OtherBodyIndex :type Integer) (bFromSweep :type Boolean) (SweepResult :type Hit%20Result%20Structure%20%28by%20ref%29))
  (if (Actor|ActorHasTag OtherActor "Person")
    (Game|Damage|ApplyDamage OtherActor (Variables|Default|GetOuterDamage) 0 0)))

(event OnComponentBeginOverlap(InnerRadius)
  (params (OverlappedComponent :type Primitive%20Component%20Object%20Reference) (OtherActor :type Actor%20Object%20Reference) (OtherComp :type Primitive%20Component%20Object%20Reference) (OtherBodyIndex :type Integer) (bFromSweep :type Boolean) (SweepResult :type Hit%20Result%20Structure%20%28by%20ref%29))
  (bind _innerwithouterdamage (Variables|Default|GetInnerWithOuterDamage))
  (if (Actor|ActorHasTag OtherActor "Person")
    (Game|Damage|ApplyDamage OtherActor _innerwithouterdamage 0 0)
    (Development|PrintString (Utilities|String|ToString(Float) _innerwithouterdamage))))

(event EventBeginPlay
  (|CallParentFunction)
  (Collision|IgnoreActorwhenMoving (Variables|Default|GetStaticMesh) (Components|GetOwner) true)
  (Collision|SetCollisionEnabled (Variables|Default|GetInnerRadius) "NoCollision")
  (Collision|SetCollisionEnabled (Variables|Default|GetOuterRadius) "NoCollision")
  (bind _asbp_assault (Utilities|Casting|CastToBP_Assault (Game|Player|GetPlayerPawn 0)))
  (Utilities|IsValid _asbp_assault
    (:Is%20Valid
      (Utilities|IsValid (Variables|/Game/_main/BluePrints/BP_Assault.BP_Assault_C|GetBP_Global_Attributes _asbp_assault)
        (:Is%20Valid
          (Utilities|IsValid (Variables|/Game/_main/BluePrints/BP_Assault.BP_Assault_C|GetBP_Grenade_Attributes _asbp_assault)
            (:Is%20Valid
              (Components|Sphere|SetSphereRadius (Variables|Default|GetInnerRadius) (* (Variables|/Script/FPSRL.BP_Global_Attributes|GetExplosivesRangeMultiplier (Variables|/Game/_main/BluePrints/BP_Assault.BP_Assault_C|GetBP_Global_Attributes _asbp_assault)) (Variables|/Script/FPSRL.BP_Throwable_Attributes|GetInnerRadius (Variables|/Game/_main/BluePrints/BP_Assault.BP_Assault_C|GetBP_Grenade_Attributes _asbp_assault))) true)
              (Components|Sphere|SetSphereRadius (Variables|Default|GetOuterRadius) (* (Variables|/Script/FPSRL.BP_Global_Attributes|GetExplosivesRangeMultiplier (Variables|/Game/_main/BluePrints/BP_Assault.BP_Assault_C|GetBP_Global_Attributes _asbp_assault)) (Variables|/Script/FPSRL.BP_Throwable_Attributes|GetOuterRadius (Variables|/Game/_main/BluePrints/BP_Assault.BP_Assault_C|GetBP_Grenade_Attributes _asbp_assault))) true)
              (Variables|Default|SetInnerWithOuterDamage (* (Variables|/Script/FPSRL.BP_Global_Attributes|GetExplosivesDamageMultiplier (Variables|/Game/_main/BluePrints/BP_Assault.BP_Assault_C|GetBP_Global_Attributes _asbp_assault)) (Variables|/Script/FPSRL.BP_Grenade_Attributes|GetInnerDamageOntopOfOuterDamage (Variables|/Game/_main/BluePrints/BP_Assault.BP_Assault_C|GetBP_Grenade_Attributes _asbp_assault))))
              (Variables|Default|SetOuterDamage (* (Variables|/Script/FPSRL.BP_Global_Attributes|GetExplosivesDamageMultiplier (Variables|/Game/_main/BluePrints/BP_Assault.BP_Assault_C|GetBP_Global_Attributes _asbp_assault)) (Variables|/Script/FPSRL.BP_Grenade_Attributes|GetOuterDamage (Variables|/Game/_main/BluePrints/BP_Assault.BP_Assault_C|GetBP_Grenade_Attributes _asbp_assault))))
              (Utilities|FlowControl|Delay 3.0)
              (Collision|SetCollisionEnabled (Variables|Default|GetInnerRadius) "QueryAndPhysics")
              (Collision|SetCollisionEnabled (Variables|Default|GetOuterRadius) "QueryAndPhysics")
              (Game|SpawnActorfromClass "/Game/_main/BluePrints/temp_blueprints/BP_Explosion.BP_Explosion_C" (Transformation|GetActorTransform) "Undefined" "MultiplyWithRoot" 0 0))))))))

(event Collision|EventActorBeginOverlap
  (params (OtherActor :type Actor%20Object%20Reference))
  (|CallParentFunction OtherActor) ; This node is disabled and will not be called.\nDrag off pins to build functionality.
)

(event EventTick
  (params (DeltaSeconds :type Float%20%28single-precision%29))
  (|CallParentFunction DeltaSeconds))

(fn ConstructionScript
  (|CallParentFunction))